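; Interactable door Blueprint that swings open when its Interact event is called; despite its name, it contains no lock or key check.
; Overlap events on the Unlock component set PlayerInteract while a ThirdPersonCharacter is near the closed door, clearing it on exit.
; Interact yaws the mesh to -90 degrees in a while loop, so it snaps open within one frame, then stays flagged IsOpen.
; OpenDoor is an empty stub.
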(event `self.Unlock.OnComponentEndOverlap`
  (params (OverlappedComponent :type "PrimitiveComponent Object Reference") (OtherActor :type "Actor Object Reference") (OtherComp :type "PrimitiveComponent Object Reference") (OtherBodyIndex :type Integer))
  (cast `/Game/ThirdPersonBP/Blueprints/ThirdPersonCharacter` OtherActor)
  (set `self.PlayerInteract` false :!label _label))

(event `self.Unlock.OnComponentBeginOverlap`
  (params (OverlappedComponent :type "PrimitiveComponent Object Reference") (OtherActor :type "Actor Object Reference") (OtherComp :type "PrimitiveComponent Object Reference") (OtherBodyIndex :type Integer) (bFromSweep :type Boolean) (SweepResult :type "HitResult Structure (by ref)"))
  (cast `/Game/ThirdPersonBP/Blueprints/ThirdPersonCharacter` OtherActor)
  (if (`self.isOpen`)
    (goto _label)
    (else
      (set `self.PlayerInteract` true))))

(event `self.Interact`
  (while (> (`self.Rotation`) -90.0)
    (bind _output_get (set `self.Rotation` (- (`self.Rotation`) 1.0)))
    (`SceneComponent.K2_SetRelativeRotation` (`self.StaticMesh`) (`KismetMathLibrary.MakeRotator` 0.0 0.0 _output_get) false false)
    (set `self.isOpen` true)
    (set `self.PlayerInteract` false)))

(fn `openDoor`)

(fn `UserConstructionScript`)