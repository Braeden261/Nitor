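; Interactable switch actor that, depending on its Type, either moves a linked elevator or calls Interact on a linked door.
; A trigger overlap with the ThirdPersonCharacter sets PlayerInteract while the switch is inactive, skipped for elevator switches when IsAtSwitch is set; leaving clears it.
; Interact sets Active and clears PlayerInteract; nothing here resets Active, so the trigger stops enabling interaction afterwards.
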(event `self.Interact`
  (set `self.Active` true)
  (set `self.PlayerInteract` false)
  (switch `int` (`self.Type`)
    (:`1`
      (`/Game/Interactables/Elevator_BP.Move Elevator` (`self.Elevator`)))
    (:`2`
      (`self.Interact` (`self.Door`)))))

(event `self.Trigger.OnComponentBeginOverlap`
  (params (OverlappedComponent :type "PrimitiveComponent Object Reference") (OtherActor :type "Actor Object Reference") (OtherComp :type "PrimitiveComponent Object Reference") (OtherBodyIndex :type Integer) (bFromSweep :type Boolean) (SweepResult :type "HitResult Structure (by ref)"))
  (cast `/Game/ThirdPersonBP/Blueprints/ThirdPersonCharacter` OtherActor)
  (if (== (`self.Type`) 1)
    (if (not (`self.IsAtSwitch`))
      (if (`self.Active`) :!label _label
        (set `self.PlayerInteract` false :!label _label_2)
        (else
          (set `self.PlayerInteract` true))))
    (else
      (goto _label))))

(event `self.Trigger.OnComponentEndOverlap`
  (params (OverlappedComponent :type "PrimitiveComponent Object Reference") (OtherActor :type "Actor Object Reference") (OtherComp :type "PrimitiveComponent Object Reference") (OtherBodyIndex :type Integer))
  (cast `/Game/ThirdPersonBP/Blueprints/ThirdPersonCharacter` OtherActor)
  (goto _label_2))

(fn `UserConstructionScript`)