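; BP_Crypt_Doorway is a two-leaf crypt door that the player can open once by interacting within its trigger.
; Overlap events on InteractTrigger1 toggle PlayerInteract for the ThirdPersonCharacter while the door is closed.
; Interact instantly rotates both leaves apart, sets IsOpen and calls SetDoors.
; An unconnected branch would reopen the door from NitorGameInstance's DoorsOpen entry for DoorNum, but never runs.
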(event `self.ReceiveBeginPlay`)

(event `self.InteractTrigger1.OnComponentBeginOverlap`
  (params (OverlappedComponent :type "PrimitiveComponent Object Reference") (OtherActor :type "Actor Object Reference") (OtherComp :type "PrimitiveComponent Object Reference") (OtherBodyIndex :type Integer) (bFromSweep :type Boolean) (SweepResult :type "HitResult Structure (by ref)"))
  (cast `/Game/ThirdPersonBP/Blueprints/ThirdPersonCharacter` OtherActor)
  (if (`self.isOpen`)
    (set `self.PlayerInteract` false :!label _label)
    (else
      (set `self.PlayerInteract` true))))

(event `self.InteractTrigger1.OnComponentEndOverlap`
  (params (OverlappedComponent :type "PrimitiveComponent Object Reference") (OtherActor :type "Actor Object Reference") (OtherComp :type "PrimitiveComponent Object Reference") (OtherBodyIndex :type Integer))
  (cast `/Game/ThirdPersonBP/Blueprints/ThirdPersonCharacter` OtherActor)
  (goto _label))

(event `self.Interact`
  (`SceneComponent.K2_AddLocalRotation` (`self.SM_DoorWay_Large_Door_Right`) (struct :`Yaw` -100.0) false false)
  (`SceneComponent.K2_AddLocalRotation` (`self.SM_DoorWay_Large_Door_Left`) (struct :`Yaw` 100.0) false false)
  (set `self.PlayerInteract` false)
  (set `self.isOpen` true)
  (`self.set Doors`))

(fn `UserConstructionScript`)