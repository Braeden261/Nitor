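; Elevator actor that moves its mesh between PointA and PointB heights when something overlaps its trigger or MoveElevator is called.
; A Direction flag alternates playing and reversing the ElevatorMovement timeline, which lerps the mesh's relative Z location without sweeping.
; An active flag blocks retriggering mid-move; on finish it clears, both switches deactivate and their IsAtSwitch flags update to match the direction.
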(event `Move Elevator`
  (bind _switcha (`self.SwitchA`))
  (bind _switchb (`self.SwitchB`))
  (if (not (`self.ElevatorActive`))
    (set `self.ElevatorActive` true)
    (`KismetSystemLibrary.PrintString` "Elevator Active")
    (if (`self.Direction`)
      (set `self.Direction` false)
      (bind (_direction _newtrack_1) (`Timeline|ElevatorMovement` :!label _label)
        (:`Update`
          (`SceneComponent.K2_SetRelativeLocation` (`self.ElevatorMesh`) (`KismetMathLibrary.VLerp` (`KismetMathLibrary.MakeVector` 0.0 0.0 (`self.PointA`)) (`KismetMathLibrary.MakeVector` 0.0 0.0 (`self.PointB`)) _newtrack_1) false false))
        (:`Finished`
          (set `self.ElevatorActive` false)
          (set `/Game/Interactables/SwitchBP.Active` false (`self.SwitchB`))
          (set `/Game/Interactables/SwitchBP.Active` false (`self.SwitchA`))
          (if (`self.Direction`)
            (set `/Game/Interactables/SwitchBP.IsAtSwitch` false _switchb)
            (set `/Game/Interactables/SwitchBP.IsAtSwitch` true _switcha)
            (else
              (set `/Game/Interactables/SwitchBP.IsAtSwitch` false _switcha)
              (set `/Game/Interactables/SwitchBP.IsAtSwitch` true _switchb)))))
      (else
        (set `self.Direction` true)
        (goto _label :!via `Reverse`)))))

(event `self.Trigger.OnComponentBeginOverlap`
  (params (OverlappedComponent :type "PrimitiveComponent Object Reference") (OtherActor :type "Actor Object Reference") (OtherComp :type "PrimitiveComponent Object Reference") (OtherBodyIndex :type Integer) (bFromSweep :type Boolean) (SweepResult :type "HitResult Structure (by ref)"))
  (`self.Move Elevator`))

(fn `UserConstructionScript`)