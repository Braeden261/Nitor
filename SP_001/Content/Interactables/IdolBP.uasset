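; Interactable idol actor that the player can use to rest.
; An Interact_Range overlap sets the PlayerInteract flag while the third-person character is inside, though Interact does not check it.
; Interact calls RestIdol on the player reference cached at BeginPlay and flags the idol interaction animation.
; A separate VisiblitySet function toggles the local fog particle system's visibility.
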(event `self.ReceiveBeginPlay`
  (bind _asthird_person_character (cast `/Game/ThirdPersonBP/Blueprints/ThirdPersonCharacter` (`GameplayStatics.GetPlayerCharacter` 0)))
  (set `self.PlayerRef` _asthird_person_character))

(event `self.ReceiveTick`
  (params (DeltaSeconds :type "Float (single-precision)")))

(event `self.interact_Range.OnComponentBeginOverlap`
  (params (OverlappedComponent :type "PrimitiveComponent Object Reference") (OtherActor :type "Actor Object Reference") (OtherComp :type "PrimitiveComponent Object Reference") (OtherBodyIndex :type Integer) (bFromSweep :type Boolean) (SweepResult :type "HitResult Structure (by ref)"))
  (cast `/Game/ThirdPersonBP/Blueprints/ThirdPersonCharacter` OtherActor)
  (set `self.PlayerInteract` true))

(event `self.interact_Range.OnComponentEndOverlap`
  (params (OverlappedComponent :type "PrimitiveComponent Object Reference") (OtherActor :type "Actor Object Reference") (OtherComp :type "PrimitiveComponent Object Reference") (OtherBodyIndex :type Integer))
  (cast `/Game/ThirdPersonBP/Blueprints/ThirdPersonCharacter` OtherActor)
  (set `self.PlayerInteract` false))

(event `self.Interact`
  (bind _playerref (`self.PlayerRef`))
  (`/Game/ThirdPersonBP/Blueprints/ThirdPersonCharacter.Rest_Idol` _playerref)
  (set `/Game/ThirdPersonBP/Blueprints/ThirdPersonCharacter.idolInteractAnimation` true _playerref))

(fn `UserConstructionScript`)

(fn `Visiblity_set`
  (`SceneComponent.ToggleVisibility` (`self.localFogParticleSystem`) false))