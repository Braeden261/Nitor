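; Boss exit door that the player can open only once the referenced boss is no longer valid.
; A trigger overlap sets PlayerInteract for the ThirdPersonCharacter when the boss reference is invalid and the door is still closed, and clears it on exit.
; The Interact event snaps both door leaves to fixed world rotations without animation, then marks the door open and non-interactable.
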(event `self.InteractTrigger1.OnComponentBeginOverlap`
  (params (OverlappedComponent :type "PrimitiveComponent Object Reference") (OtherActor :type "Actor Object Reference") (OtherComp :type "PrimitiveComponent Object Reference") (OtherBodyIndex :type Integer) (bFromSweep :type Boolean) (SweepResult :type "HitResult Structure (by ref)"))
  (cast `/Game/ThirdPersonBP/Blueprints/ThirdPersonCharacter` OtherActor)
  (`/Engine/EditorBlueprintResources/StandardMacros.IsValid` (`self.BossRef`)
    (:`Is Valid`
      (set `self.PlayerInteract` false :!label _label))
    (:`Is Not Valid`
      (if (`self.isOpen`)
        (goto _label)
        (else
          (set `self.PlayerInteract` true))))))

(event `self.InteractTrigger1.OnComponentEndOverlap`
  (params (OverlappedComponent :type "PrimitiveComponent Object Reference") (OtherActor :type "Actor Object Reference") (OtherComp :type "PrimitiveComponent Object Reference") (OtherBodyIndex :type Integer))
  (cast `/Game/ThirdPersonBP/Blueprints/ThirdPersonCharacter` OtherActor)
  (goto _label))

(event `self.Interact`
  (`SceneComponent.K2_SetWorldRotation` (`self.SM_DoorWay_Large_Door_Right`) (struct :`Yaw` -110.0) false false)
  (`SceneComponent.K2_SetWorldRotation` (`self.SM_DoorWay_Large_Door_Left`) (struct :`Yaw` 110.0) false false)
  (set `self.isOpen` true)
  (set `self.PlayerInteract` false))

(fn `UserConstructionScript`)