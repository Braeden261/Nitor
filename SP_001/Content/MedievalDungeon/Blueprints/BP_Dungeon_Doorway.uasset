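; Dungeon doorway Blueprint with a pair of large doors that open once through an Interact event.
; Box overlaps with ThirdPersonCharacter set a PlayerInteract flag while the doors are closed, and clear it on exit or once open.
; Interact, triggered from outside this graph, snaps both door meshes to hard-coded world rotations, independent of actor orientation, and sets IsOpen.
; There is no animation or closing logic.
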(event `self.Box.OnComponentBeginOverlap`
  (params (OverlappedComponent :type "PrimitiveComponent Object Reference") (OtherActor :type "Actor Object Reference") (OtherComp :type "PrimitiveComponent Object Reference") (OtherBodyIndex :type Integer) (bFromSweep :type Boolean) (SweepResult :type "HitResult Structure (by ref)"))
  (cast `/Game/ThirdPersonBP/Blueprints/ThirdPersonCharacter` OtherActor)
  (if (`self.isOpen`)
    (set `self.PlayerInteract` false :!label _label)
    (else
      (set `self.PlayerInteract` true))))

(event `self.Box.OnComponentEndOverlap`
  (params (OverlappedComponent :type "PrimitiveComponent Object Reference") (OtherActor :type "Actor Object Reference") (OtherComp :type "PrimitiveComponent Object Reference") (OtherBodyIndex :type Integer))
  (cast `/Game/ThirdPersonBP/Blueprints/ThirdPersonCharacter` OtherActor)
  (goto _label))

(event `self.Interact`
  (`SceneComponent.K2_SetWorldRotation` (`self.SM_DoorWay_Large_Door_Right`) (struct :`Yaw` 180.0) false false)
  (`SceneComponent.K2_SetWorldRotation` (`self.SM_DoorWay_Large_Door_Left`) (struct) false false)
  (set `self.isOpen` true))

(fn `UserConstructionScript`)